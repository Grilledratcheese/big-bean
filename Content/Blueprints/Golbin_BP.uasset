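; Golbin_BP is an AI-moved pawn that follows the BP_Leigh character.
; On BeginPlay it finds and caches that actor, then issues a single AI MoveTo with it as target actor, which takes precedence over the supplied offset destination.
; Tick keeps storing the player's location in PlayerPOS, but the move is never reissued with the updated value.
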(event `FollowPlayer`
  (bind _returnvalue (`GameplayStatics.GetActorOfClass` "/Game/Blueprints/BP_Leigh.BP_Leigh_C"))
  (bind _output_get (set `self.CharRef` _returnvalue))
  (`|AIMoveTo` self (- (`self.PlayerPOS`) (100.0 100.0 0.0)) _output_get))

(event `Get Player POS`
  (set `self.PlayerPOS` (`self.K2_GetActorLocation` (`self.CharRef`))))

(event `self.ReceiveTick`
  (params (DeltaSeconds :type "Float (single-precision)"))
  (`self.Get Player POS`))

(event `self.ReceiveBeginPlay`
  (`self.FollowPlayer`))

(fn `UserConstructionScript`)