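; BP_Leigh is a player-controllable pawn that destroys any BP_Wiley actor that touches its Box component.
; Axis inputs drive movement along the actor's forward and right vectors, with forced movement input, and feed controller pitch and yaw for looking.
; The Box begin-overlap event casts the other actor to BP_Wiley and destroys it, ignoring all other actors.
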(event `InputAxis|walk`
  (params (AxisValue :type "Float (single-precision)"))
  (`self.AddMovementInput` (`self.GetActorForwardVector`) AxisValue true))

(event `InputAxis|lookup`
  (params (AxisValue :type "Float (single-precision)"))
  (`self.AddControllerPitchInput` AxisValue))

(event `InputAxis|lookright`
  (params (AxisValue :type "Float (single-precision)"))
  (`self.AddControllerYawInput` AxisValue))

(event `InputAxis|right`
  (params (AxisValue :type "Float (single-precision)"))
  (`self.AddMovementInput` (`self.GetActorRightVector`) AxisValue true))

(event `self.Box.OnComponentBeginOverlap`
  (params (OverlappedComponent :type "PrimitiveComponent Object Reference") (OtherActor :type "Actor Object Reference") (OtherComp :type "PrimitiveComponent Object Reference") (OtherBodyIndex :type Integer) (bFromSweep :type Boolean) (SweepResult :type "HitResult Structure (by ref)"))
  (bind _asbp_wiley (cast `/Game/Blueprints/BP_Wiley` OtherActor))
  (`self.K2_DestroyActor` _asbp_wiley))

(fn `UserConstructionScript`)