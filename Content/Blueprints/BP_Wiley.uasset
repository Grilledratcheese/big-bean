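; BP_Wiley is an AI follower that pursues the BP_Leigh actor, treated as the player.
; From BeginPlay, FollowPlayer looks up that actor, issues AIMoveTo toward it, then calls itself after a short delay to keep re-pathing.
; Tick caches the player's location for an offset Destination, though the move also passes the player as TargetActor, which takes precedence over that point.
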(event `FollowPlayer`
  (bind _returnvalue (`GameplayStatics.GetActorOfClass` "/Game/Blueprints/BP_Leigh.BP_Leigh_C"))
  (bind _output_get (set `self.PlayerRef` _returnvalue))
  (`|AIMoveTo` self (- (stale `GetPlayerPOS` _output_get) (100.0 100.0 0.0)) _output_get 100.0
    (:`then`
      (`KismetSystemLibrary.Delay` 0.2)
      (`self.FollowPlayer`))))

(event `GetPlayerPOS`
  (bind _output_get (set `self.PlayerPOS` (`self.K2_GetActorLocation` (`self.PlayerRef`)))))

(event `self.ReceiveBeginPlay`
  (`self.FollowPlayer`))

(event `self.ReceiveTick`
  (params (DeltaSeconds :type "Float (single-precision)"))
  (`self.GetPlayerPOS`))

(fn `UserConstructionScript`)